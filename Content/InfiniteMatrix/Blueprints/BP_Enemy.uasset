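; BP_Enemy is an enemy actor that reacts to overlaps on its EnemyHitbox component.
; When a BP_Projectile hits it, it adds five to the score on the firing player's HUD widget, then destroys both the projectile and itself.
; When it touches a BP_Player instead, it destroys itself and deals damage to that player.
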(event `self.EnemyHitbox.OnComponentBeginOverlap`
  (params (OverlappedComponent :type "PrimitiveComponent Object Reference") (OtherActor :type "Actor Object Reference") (OtherComp :type "PrimitiveComponent Object Reference") (OtherBodyIndex :type Integer) (bFromSweep :type Boolean) (SweepResult :type "HitResult Structure (by ref)"))
  (bind _asbp_projectile (cast `/Game/InfiniteMatrix/Blueprints/BP_Projectile` OtherActor)
    (:`then`
      (bind _hudwidget (`/Game/InfiniteMatrix/Blueprints/BP_Player.HUDWidget` (`/Game/InfiniteMatrix/Blueprints/BP_Projectile.Player` _asbp_projectile)))
      (`/Game/InfiniteMatrix/UI/WBP_HUD.SetScore` _hudwidget (+ 5 (`/Game/InfiniteMatrix/UI/WBP_HUD.Score` _hudwidget)))
      (`self.K2_DestroyActor` _asbp_projectile)
      (`self.K2_DestroyActor`))
    (:`CastFailed`
      (bind _asbp_player (cast `/Game/InfiniteMatrix/Blueprints/BP_Player` OtherActor))
      (`self.K2_DestroyActor`)
      (`/Game/InfiniteMatrix/Blueprints/BP_Player.TakeDamage` _asbp_player 10.0))))

(fn `UserConstructionScript`)