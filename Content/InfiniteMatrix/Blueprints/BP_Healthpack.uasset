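; BP_Healthpack is a health pickup that reacts to overlaps on its HealthpackCollect component.
; A BP_Player overlap adds a small fixed amount of health, clamped to the maximum, refreshes the player's HUD health bar, then destroys the pickup.
; A BP_Projectile overlap destroys both the projectile and the pickup without healing, so shots can eliminate healthpacks.
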(event `self.HealthpackCollect.OnComponentBeginOverlap`
  (params (OverlappedComponent :type "PrimitiveComponent Object Reference") (OtherActor :type "Actor Object Reference") (OtherComp :type "PrimitiveComponent Object Reference") (OtherBodyIndex :type Integer) (bFromSweep :type Boolean) (SweepResult :type "HitResult Structure (by ref)"))
  (bind _asbp_player (cast `/Game/InfiniteMatrix/Blueprints/BP_Player` OtherActor)
    (:`then`
      (bind _output_get (set `/Game/InfiniteMatrix/Blueprints/BP_Player.Health` (`KismetMathLibrary.FClamp` (+ 5.0 (`/Game/InfiniteMatrix/Blueprints/BP_Player.Health` _asbp_player)) 0.0 100.0) _asbp_player))
      (`/Game/InfiniteMatrix/UI/WBP_HUD.SetHealthBarInfo` (`/Game/InfiniteMatrix/Blueprints/BP_Player.HUDWidget` _asbp_player) _output_get 100.0)
      (`self.K2_DestroyActor`))
    (:`CastFailed`
      (bind _asbp_projectile (cast `/Game/InfiniteMatrix/Blueprints/BP_Projectile` OtherActor))
      (`self.K2_DestroyActor` _asbp_projectile)
      (`self.K2_DestroyActor`))))

(fn `UserConstructionScript`)